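; BP_BaseCharacter is a base character that sets up its player's HUD, team skin, scoreboard and replay hotkeys.
; On BeginPlay it adds the in-game HUD if locally controlled and picks the mesh material from PlayerSkins using the player state's TeamColor.
; Holding Tab shows the scoreboard widget.
; Number keys start and stop recording and start replay through BaseGameInstance, or restart recording through MasterPlayerController.
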(event EventBeginPlay
  (Utilities|FlowControl|Sequence
    (:then_0
      (if (Pawn|IsLocallyControlled)
        (bind _returnvalue (UserInterface|CreateWidget "/Game/UI/InGameHUD.InGameHUD_C"))
        (UserInterface|Viewport|AddtoViewport _returnvalue 0)))
    (:then_1
      (bind _asbase_player_state (Utilities|Casting|CastToBasePlayerState (Variables|Default|GetPlayerState)))
      (Rendering|Material|SetMaterial (Variables|Character|GetMesh) 0 (Utilities|Array|Get(acopy) (Variables|Default|GetPlayerSkins) (Variables|/Script/SilentRed.BasePlayerState|GetTeamColor _asbase_player_state))))))

(event Input|KeyboardEvents|1
  (params (Key :type Key%20Structure :default "None"))
  (:Pressed
    (bind _asbase_game_instance (Utilities|Casting|CastToBaseGameInstance (Game|GetGameInstance)))
    (Class|BaseGameInstance|StartRecording _asbase_game_instance)))

(event Input|KeyboardEvents|2
  (params (Key :type Key%20Structure :default "None"))
  (:Pressed
    (bind _asbase_game_instance (Utilities|Casting|CastToBaseGameInstance (Game|GetGameInstance)))
    (Class|BaseGameInstance|StopRecording _asbase_game_instance)))

(event Input|KeyboardEvents|3
  (params (Key :type Key%20Structure :default "None"))
  (:Pressed
    (bind _asbase_game_instance (Utilities|Casting|CastToBaseGameInstance (Game|GetGameInstance)))
    (Class|BaseGameInstance|StartReplay _asbase_game_instance)))

(event Input|KeyboardEvents|4
  (params (Key :type Key%20Structure :default "None"))
  (:Pressed
    (bind _asmaster_player_controller (Utilities|Casting|CastToMasterPlayerController (Game|GetPlayerController 0)))
    (Class|MasterPlayerController|RestartRecording _asmaster_player_controller)))

(event Input|KeyboardEvents|Tab
  (params (Key :type Key%20Structure :default "None"))
  (:Pressed
    (bind _returnvalue (UserInterface|CreateWidget "/Game/UI/MenuSystem/BP_ScoreBoard.BP_ScoreBoard_C" (Game|GetPlayerController 0)))
    (UserInterface|Viewport|AddtoViewport _returnvalue 0))
  (:Released
    (Widget|RemovefromParent _returnvalue)))

(fn ConstructionScript)